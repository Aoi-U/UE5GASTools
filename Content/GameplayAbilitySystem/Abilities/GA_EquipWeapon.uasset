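; Gameplay ability that equips a staff or sword on the avatar in response to a gameplay event.
; It commits, then switches on the first target tag in the event data to pick the weapon Blueprint class for the avatar's WeaponsManagerComponent to equip.
; It ends after the switch, but only inside the valid-component branch, so a missing component leaves the ability active.
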(event `self.K2_ActivateAbilityFromEvent`
  (params (EventData :type "GameplayEventData Structure (by ref)"))
  (bind _returnvalue (`Actor.GetComponentByClass` (`self.GetAvatarActorFromActorInfo`) "/Game/Weapons/WeaponsManagerComponent.WeaponsManagerComponent_C"))
  (`self.K2_CommitAbility`)
  (`/Engine/EditorBlueprintResources/StandardMacros.IsValid` _returnvalue
    (:`Is Valid`
      (`|ExecutionSequence`
        (:`then_0`
          (`|SwitchGameplayTag` (`|GetArrayItem` (`BlueprintGameplayTagLibrary.BreakGameplayTagContainer` (`.TargetTags` (break `GameplayEventData` EventData))))
            (:`Weapon.Ranged.Staff`
              (`/Game/Weapons/WeaponsManagerComponent.EquipWeapon` _returnvalue "/Game/Weapons/BP_Weapon_Staff.BP_Weapon_Staff_C"))
            (:`Weapon.Melee.Sword`
              (`/Game/Weapons/WeaponsManagerComponent.EquipWeapon` _returnvalue "/Game/Weapons/BP_Weapon_Sword.BP_Weapon_Sword_C"))))
        (:`then_1`
          (`self.K2_EndAbility`))))))